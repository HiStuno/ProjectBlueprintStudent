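; Interactive mesh actor that lets the player switch its material from within a trigger box.
; Entering or leaving the box enables or disables player input and toggles visibility of the TextRender and Reset components.
; E steps a MultiGate through the scrolls, apple and bed material instances on the mesh's first slot.
; R resets the gate sequence without itself changing the current material.
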(event OnComponentBeginOverlap(Box)
  (params (OverlappedComponent :type Primitive%20Component%20Object%20Reference) (OtherActor :type Actor%20Object%20Reference) (OtherComp :type Primitive%20Component%20Object%20Reference) (OtherBodyIndex :type Integer) (bFromSweep :type Boolean) (SweepResult :type Hit%20Result%20Structure%20%28by%20ref%29))
  ;[0 0 0] Visibility Bouton
  (Input|EnableInput (Game|GetPlayerController 0))
  (Rendering|ToggleVisibility (Variables|Default|GetTextRender) false))

(event OnComponentEndOverlap(Box)
  (params (OverlappedComponent :type Primitive%20Component%20Object%20Reference) (OtherActor :type Actor%20Object%20Reference) (OtherComp :type Primitive%20Component%20Object%20Reference) (OtherBodyIndex :type Integer))
  ;[0 0 0] Visibility Bouton
  (Input|DisableInput (Game|GetPlayerController 0))
  (Rendering|ToggleVisibility (Variables|Default|GetTextRender) false))

(event EventBeginPlay)

(event Collision|EventActorBeginOverlap
  (params (OtherActor :type Actor%20Object%20Reference)))

(event EventTick
  (params (DeltaSeconds :type Float%20%28single-precision%29)))

(event Input|KeyboardEvents|E
  (params (Key :type Key%20Structure :default "None"))
  ;[0 0 0] Change Mat
  (:Pressed
    (Utilities|FlowControl|MultiGate false false -1
      (:Out%200
        (Rendering|Material|SetMaterial (Variables|Default|GetStaticMeshComponent0) 0 "/Game/AlchemistsHouse/Assets/Materials/Instances/MI_Scrolls.MI_Scrolls"))
      (:Out%201
        (Rendering|Material|SetMaterial (Variables|Default|GetStaticMeshComponent0) 0 "/Game/AlchemistsHouse/Assets/Materials/Instances/MI_Apple.MI_Apple"))
      (:Out%202
        (Rendering|Material|SetMaterial (Variables|Default|GetStaticMeshComponent0) 0 "/Game/AlchemistsHouse/Assets/Materials/Instances/MI_Bed.MI_Bed")))))

(event Input|KeyboardEvents|R
  (params (Key :type Key%20Structure :default "None"))
  ;[0 0 0] Change Mat
  (:Pressed
    (Utilities|FlowControl|MultiGate false false -1) ; enters at Reset
  ))

(fn ConstructionScript)